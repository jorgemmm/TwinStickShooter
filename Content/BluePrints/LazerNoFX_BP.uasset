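; Laser projectile Blueprint that damages non-friendly actors it overlaps.
; On overlap, actors implementing IDamageable without the "Friendly" tag receive damage through an interface message, then an explosion sound and spark emitter spawn and the projectile is destroyed.
; Overlapping a non-damageable actor destroys it after a short delay without effects, while friendly damageable actors are ignored.
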(event `self.ReceiveActorBeginOverlap`
  (params (OtherActor :type "Actor Object Reference"))
  (bind (_returnvalue_location _returnvalue_rotation) (`KismetMathLibrary.BreakTransform` (`self.GetTransform`)))
  ;[1 1 1] Handle Projectile overlap with actor with interfase idamageable - Damage  by interfase - Spawn sparks  - destroy projectile
  (if (`KismetSystemLibrary.DoesImplementInterface` OtherActor "/Game/BluePrints/iDamageable.iDamageable_C")
    (if (not (`self.ActorHasTag` OtherActor "Friendly"))
      (message `/Game/BluePrints/iDamageable.AffectHealth` OtherActor (`self.Damage`)) ; Provoca 20 de daño através de la interfase
      (`GameplayStatics.SpawnSoundAttached` "/Game/StarterContent/Audio/Explosion01.Explosion01" (`self.ProjecileCollision`) "None" (0.0 0.0 0.0) (struct) "KeepRelativeOffset" false 1.0 1.0 0.0 null null)
      (`GameplayStatics.SpawnEmitterAtLocation` "/Game/StarterContent/Particles/LazerSparks.LazerSparks" _returnvalue_location _returnvalue_rotation) ; Sólo si colisiona con enemy
      (`self.K2_DestroyActor` :!label _label) ; Destruye el proyectil
    )
    (else
      (`KismetSystemLibrary.Delay` 1.0)
      (goto _label))))

(event `self.ProjecileCollision.OnComponentHit`
  (params (HitComponent :type "PrimitiveComponent Object Reference") (OtherActor :type "Actor Object Reference") (OtherComp :type "PrimitiveComponent Object Reference") (NormalImpulse :type "Vector Structure") (Hit :type "HitResult Structure (by ref)"))
  ;[1 1 1] Handle Projectile overlap with actor with interfase idamageable - Damage  by interfase - Spawn sparks  - destroy projectile
)

(fn `UserConstructionScript`)