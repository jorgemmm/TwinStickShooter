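; Zombie enemy for a twin-stick shooter that damages the hero on contact and scores points when killed.
; Overlapping BP_HeroApocaGirl starts a looping damage timer at its attack rate, cleared when overlap ends.
; AffectHealth plays random pain sounds; death disables projectile and pawn collision, increments game-mode score, detaches the controller, spawns an explosion and destroys the actor.
; Tick updates a player-facing health bar; construction tints the body via dynamic material.
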(event `self.ReceiveBeginPlay`
  ;[1 1 1] Setting the maxSpeed
  (set `CharacterMovementComponent.MaxWalkSpeed` (`self.MaxEnemySpeed`) (`self.CharacterMovement`)))

(event `/Game/BluePrints/iDamageable.AffectHealth`
  (params (Delta :type "Float (single-precision)"))
  (bind _arraypainau (`self.ArrayPainAU`))
  (bind _arraypaindeath (`self.ArrayPainDeath`))
  (bind _capsulecomponent (`self.CapsuleComponent`))
  ;[1 1 1] Damaging Enemy  (By Hero Projetile)
  (`self.CalculateHealth` Delta)
  (if (`self.isDead`)
    (`PrimitiveComponent.SetCollisionResponseToChannel` _capsulecomponent "ECC_WorldDynamic" "ECR_Ignore" :!pinned true) ; De esta forma el enemgo caído ignora los proyectiles
    (`PrimitiveComponent.SetCollisionResponseToChannel` _capsulecomponent "ECC_Pawn" "ECR_Ignore" :!pinned true) ; Y al Hero, aunque podría ser útil que los cuerpos entorpecieran el mvto, poner block entonces
    (bind _astwin_stick_gm (cast `/Game/BluePrints/TwinStickGM` (`GameplayStatics.GetGameMode`)))
    (`/Game/BluePrints/TwinStickGM.IncrementScore` _astwin_stick_gm (`self.Score`))
    (`self.DetachFromControllerPendingDestroy` :!pinned true) ; Este nodo es más especifico, elimina el controlador
    ;[1 1 1] Enemy sounds Aghhhh why
    (`GameplayStatics.PlaySoundAtLocation` (`|GetArrayItem` _arraypaindeath (`KismetMathLibrary.RandomIntegerInRange` 0 (`KismetArrayLibrary.Array_LastIndex` _arraypaindeath))) (`self.K2_GetActorLocation`) (struct) 1.0 1.0 0.0 null null null)
    (`|SpawnActorFromClass` "/Game/BluePrints/Explosion.Explosion_C" (`self.GetTransform`) "Undefined" "OverrideRootScale" null null)
    (`KismetSystemLibrary.Delay` 2.0)
    (`self.K2_DestroyActor`)
    (else
      ;[1 1 1] Enemy Sounds Auuu
      (`GameplayStatics.PlaySoundAtLocation` (`|GetArrayItem` _arraypainau (`KismetMathLibrary.RandomIntegerInRange` 0 (`KismetArrayLibrary.Array_LastIndex` _arraypainau))) (`self.K2_GetActorLocation`) (struct) 1.0 1.0 0.0 null null null))))

(event `self.ReceiveTick`
  (params (DeltaSeconds :type "Float (single-precision)"))
  (bind _returnvalue (`GameplayStatics.GetPlayerCharacter` 0))
  ;[1 1 1] Show Health Bar
  (bind _ashealth_bar_enemy (cast `/Game/HUD/HealthBarEnemy` (`WidgetComponent.GetUserWidgetObject` (`self.HealthWG`))))
  (`ProgressBar.SetPercent` (`/Game/HUD/HealthBarEnemy.HealthProgressBar` _ashealth_bar_enemy) (/ (`self.Health`) 100.0))
  (bind _asbp_hero_character (cast `/Game/BluePrints/BP_HeroCharacter` _returnvalue))
  (if (not (`BaseCharacter.isDead` _asbp_hero_character))
    (`SceneComponent.K2_SetWorldRotation` (`self.HealthWG`) (`KismetMathLibrary.MakeRotator` 0.0 (`self.ToSeeFromAir`) (.yaw (`KismetMathLibrary.FindLookAtRotation` (`SceneComponent.K2_GetComponentLocation` (`self.HealthWG`)) (`self.K2_GetActorLocation` _returnvalue)))) false false)))

(event `self.ReceiveActorBeginOverlap`
  (params (OtherActor :type "Actor Object Reference"))
  ;[1 1 1] Damaging Hero by Collision using interfase
  (bind _asbp_hero_apoca_girl (cast `/Game/BluePrints/Girl/BP_HeroApocaGirl` OtherActor))
  (set `self.HeroGirl` _asbp_hero_apoca_girl)
  (`KismetSystemLibrary.K2_SetTimer` null "DamageTheHero" (/ 1.0 (`self.AttackPerSeconds`)) true)
  (set `self.bIsAtacking` true))

(event `self.ReceiveActorEndOverlap`
  (params (OtherActor :type "Actor Object Reference"))
  ;[1 1 1] Damaging Hero by Collision using interfase
  (if (== OtherActor (`self.HeroGirl`))
    (`KismetSystemLibrary.K2_ClearTimer` null "DamageTheHero")
    (set `self.bIsAtacking` false)))

(event `DamageTheHero`
  ;[1 1 1] Damaging Hero by Collision using interfase
  (`/Game/BluePrints/iDamageable.AffectHealth` (`self.HeroGirl`) (`self.Damage`)))

(fn `UserConstructionScript`
  (bind _returnvalue (`PrimitiveComponent.CreateDynamicMaterialInstance` (`self.Mesh`) 0 null "None"))
  (bind _output_get (set `self.DynaMat` _returnvalue))
  (`MaterialInstanceDynamic.SetVectorParameterValue` _output_get "BodyColor" (`self.EnemyColor`)))