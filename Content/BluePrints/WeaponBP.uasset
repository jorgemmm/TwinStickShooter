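; Weapon Blueprint that fires a three-way spread of projectiles while the trigger is held.
; PullTrigger fires once through a DoOnce, then loops Fire on a timer set by RoundsPerSecond; ReleaseTrigger clears the timer and resets the gate.
; Each shot spawns projectiles at ProjectileSpawnPoint, straight and yawed by ±AngleSpawn, each with a random class from ProjetileKind.
; The LaserFire sound node is disconnected and never plays.
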(event `PullTrigger`
  ;[1 1 1] Firing with Trigger buttons
  (`/Engine/EditorBlueprintResources/StandardMacros.DoOnce` false :!label _label
    (:`Completed`
      (`self.Fire`)
      (`KismetSystemLibrary.K2_SetTimer` null "Fire" (/ 1.0 (`self.RoundsPerSeconds`)) true))))

(event `ReleaseTrigger`
  ;[1 1 1] Firing with Trigger buttons
  (`KismetSystemLibrary.K2_ClearTimer` null "Fire")
  (goto _label :!via `Reset`))

(event `Fire`
  (bind _projetilekind (`self.ProjetileKind`))
  (bind _centralspawnpoint (`self.CentralSpawnPoint`))
  (bind _centralspawnpoint_2 (`self.CentralSpawnPoint`))
  (bind _output (`|GetArrayItem` _projetilekind (`KismetMathLibrary.RandomIntegerInRange` 0 (`KismetArrayLibrary.Array_LastIndex` _projetilekind))))
  ;[1 1 1] Firing with Trigger buttons
  (bind _output_get (set `self.CentralSpawnPoint` (`SceneComponent.K2_GetComponentToWorld` (`self.ProjectileSpawnPoint`))))
  (`|SpawnActorFromClass` _output _output_get "Undefined" "OverrideRootScale" null null)
  (bind _output_get_2 (set `self.LeftSpawnPont` (`KismetMathLibrary.MakeTransform` (.location _centralspawnpoint_2) (`KismetMathLibrary.MakeRotator` (.roll (.rotation _centralspawnpoint_2)) (.pitch (.rotation _centralspawnpoint_2)) (+ (.yaw (.rotation _centralspawnpoint_2)) (`self.AngleSpawn`))) (.scale _centralspawnpoint_2))))
  (`|SpawnActorFromClass` _output _output_get_2 "Undefined" "OverrideRootScale" null null)
  (bind _output_get_3 (set `self.RightSpawnPoint` (`KismetMathLibrary.MakeTransform` (.location _centralspawnpoint) (`KismetMathLibrary.MakeRotator` (.roll (.rotation _centralspawnpoint)) (.pitch (.rotation _centralspawnpoint)) (- (.yaw (.rotation _centralspawnpoint)) (`self.AngleSpawn`))) (.scale _centralspawnpoint))))
  (`|SpawnActorFromClass` _output _output_get_3 "Undefined" "OverrideRootScale" null null))

(fn `UserConstructionScript`)