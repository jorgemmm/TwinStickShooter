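; Game mode for a zombie shooter that drives enemy spawning, hero respawn and score.
; On BeginPlay it finds the first woman and man zombie spawners and starts looping timers that call their SpawnEnemy function at a rate set by EnemyPerSeconds.
; RespawnPlayer destroys all enemies, then after a short delay spawns and possesses a new BP_HeroApocaGirl.
; IncrementScore adds to Score, while SetRoundPerSeconds is an empty stub.
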(event `self.ReceiveBeginPlay`
  ;[1 1 1] Enemy Spawn : Zombie spawnwers
  (`|ExecutionSequence`
    (:`then_0`
      (bind _outactors (`GameplayStatics.GetAllActorsOfClass` "/Game/BluePrints/Zombies/ZombieWoManSpawner.ZombieWomanSpawner_C"))
      (bind _output_get (set `self.ZWomanSpawner` (`|GetArrayItem` _outactors)))
      (`KismetSystemLibrary.K2_SetTimer` _output_get "SpawnEnemy" (/ 1.0 (`self.EnemyPerSeconds`)) true) ; Toma la función del object, Spawner
    )
    (:`then_1`
      (bind _outactors_2 (`GameplayStatics.GetAllActorsOfClass` "/Game/BluePrints/Zombies/ZombieManSpawner.ZombieManSpawner_C"))
      (bind _output_get_2 (set `self.ZManSpawner` (`|GetArrayItem` _outactors_2)))
      (`KismetSystemLibrary.K2_SetTimer` _output_get_2 "SpawnEnemy" (/ 1.0 (`self.EnemyPerSeconds`)) true) ; Toma la función del object, Spawner
    )))

(event `RespawnPlayer`
  ;[1 1 1] Hero Spawn
  (bind _outactors (`GameplayStatics.GetAllActorsOfClass` "/Game/BluePrints/Zombies/BP_BaseEnemyZ.BP_BaseEnemyZ_C"))
  (for _array_element _outactors
    (`self.K2_DestroyActor` _array_element))
  (`KismetSystemLibrary.Delay` 0.5)
  (bind _returnvalue (`|SpawnActorFromClass` "/Game/BluePrints/Girl/BP_HeroApocaGirl.BP_HeroApocaGirl_C" (`self.GirlApocaSpawnTransform`) "Undefined" "OverrideRootScale" null null))
  (`Controller.Possess` (`GameplayStatics.GetPlayerController` 0) _returnvalue))

(event `IncrementScore`
  (params (DeltaScore :type Integer))
  ;[1 1 1] Score Increment
  (set `self.Score` (+ DeltaScore (`self.Score`))))

(event `SetRoundPerSeconds`)

(fn `UserConstructionScript`)